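; BP_TPC is a character Blueprint that plays hit animations when the 1 key is pressed.
; The key press plays the mannequin montage from a randomly chosen section, building the name by appending a random number to "Hit".
; An unconnected montage-is-playing check has no effect, so nothing in the graph guards against replaying mid-animation.
; The default events are disabled and the construction script only calls its parent.
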(event EventBeginPlay
  (|CallParentFunction) ; This node is disabled and will not be called.\nDrag off pins to build functionality.
)

(event Collision|EventActorBeginOverlap
  (params (OtherActor :type Actor%20Object%20Reference))
  (|CallParentFunction OtherActor) ; This node is disabled and will not be called.\nDrag off pins to build functionality.
)

(event EventTick
  (params (DeltaSeconds :type Float%20%28single-precision%29))
  (|CallParentFunction DeltaSeconds) ; This node is disabled and will not be called.\nDrag off pins to build functionality.
)

(event Input|KeyboardEvents|1
  (params (Key :type Key%20Structure :default "None"))
  (:Pressed
    (Animation|PlayAnimMontage "/Game/AnimStarterPack/UE4_Mannequin/Mesh/UE4_Mannequin_Skeleton_Montage.UE4_Mannequin_Skeleton_Montage" 1.0 (Utilities|String|StringToName (Utilities|String|Append "Hit" (Utilities|String|ToString(Integer) (Class|KismetMathLibrary|RandomInteger64inRange 1 4)))))))

(fn ConstructionScript
  (|CallParentFunction))